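; Base drivable car Blueprint that feeds player input to BPEngineComponent and layers cameras, audio, nitrox and drifting on top.
; Tick drives speed-curve FOV, camera angle and radial blur, idle orbit and look-behind, plus FMOD engine parameters from load and RPM.
; Nitrox uses a gated boost force with fuel, duration and scaled cooldown.
; Velocity slip flags drifting wheels; particle and nitrox-material functions are empty stubs.
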(event `self.ReceiveBeginPlay`
  (`self.BeginPlayAudio`)
  (`self.BeginPlaySetupNitrox`)
  (`self.BeginPlaySetupPostProcessMaterial`)
  (`self.BeginPlayManualGearShift`)
  (`self.StartCameraShake`)
  (`self.ApplyEngineComponentSettings`))

(event `ApplyEngineComponentSettings`
  (bind _bp_enginecomponent (`self.BP_EngineComponent`))
  (set `/Game/Core/Vehicles/BP_EngineComponent.EngineSettings` (`self.EngineSettings`) _bp_enginecomponent)
  (set `/Game/Core/Vehicles/BP_EngineComponent.NitroxSettings` (`self.NitroxSettings`) _bp_enginecomponent)
  (set `/Game/Core/Vehicles/BP_EngineComponent.TurboSettings` (`self.TurboSettings`) _bp_enginecomponent))

(event `self.ReceiveTick`
  (params (DeltaSeconds :type "Float (single-precision)"))
  (bind _bp_enginecomponent (`self.BP_EngineComponent`))
  (`|ExecutionSequence`
    (:`then_0`
      (if (`self.TickReadPlayerInput`)
        (`self.TickCollectInputs`)))
    (:`then_1`
      (`self.TickCameraFOV`)
      (`self.TickCameraAngle`)
      (`self.TickRadialBlurIntensity`)
      (`self.Tick3rdPersonCameraRotation`)
      (`self.Tick1stPersonCameraRotation`))
    (:`then_2`
      (`self.TickAudio`))
    (:`then_3`
      (`self.TickNitroxCooldown`)
      (`self.TickNitrox`)
      (`self.UpdateNitroxUpDirection`))
    (:`then_4`
      (`self.TickUpdateDrifting`))
    (:`then_5`
      (`/Game/Core/Vehicles/BP_EngineComponent.InputThrottle` _bp_enginecomponent (`self.ThrottleInput`))
      (`/Game/Core/Vehicles/BP_EngineComponent.InputSteering` _bp_enginecomponent (`self.SteeringInput`)))))

(event `TickRadialBlurIntensity`
  (bind _dynamicradialblur (`self.DynamicRadialBlur`))
  (bind _bp_enginecomponent (`self.BP_EngineComponent`))
  (`/Engine/EditorBlueprintResources/StandardMacros.IsValid` _dynamicradialblur
    (:`Is Valid`
      (`MaterialInstanceDynamic.SetScalarParameterValue` _dynamicradialblur "BlurStrength" (`KismetMathLibrary.GetRuntimeFloatCurveValue` (`/Game/Core/Vehicles/PDA_CameraSettings.RadialBlurIntensityOverSpeed` (`self.CameraSettings`)) (/ (`/Game/Core/Vehicles/BP_EngineComponent.CurrentSpeed` _bp_enginecomponent) (`/Game/Core/Vehicles/PDA_EngineSettings.MaxSpeed` (`/Game/Core/Vehicles/BP_EngineComponent.EngineSettings` _bp_enginecomponent))))))))

(event `BeginPlaySetupPostProcessMaterial`
  ;[1 1 1] Dynamic post processing shader to apply blur to the edge of the screen when moving quickly
  (bind _returnvalue (`KismetMaterialLibrary.CreateDynamicMaterialInstance` "/Game/Art/Materials/PostProcess/PPM_RadialBlur.PPM_RadialBlur"))
  (bind _output_get (set `self.DynamicRadialBlur` _returnvalue))
  (`KismetArrayLibrary.Array_Add` (`.Array` (break `WeightedBlendables` (`.WeightedBlendables` (break `PostProcessSettings` (`CameraComponent.PostProcessSettings` (`self.3rdPersonCamera`)))))) (make `WeightedBlendable` 1.0 _output_get)))

(event `TickCameraFOV`
  (bind _camerasettings (`self.CameraSettings`))
  (`CameraComponent.SetFieldOfView` (`self.3rdPersonCamera`) (`KismetMathLibrary.GetRuntimeFloatCurveValue` (`/Game/Core/Vehicles/PDA_CameraSettings.FOVOverSpeed` _camerasettings) (/ (`/Game/Core/Vehicles/BP_EngineComponent.CurrentSpeed` (`self.BP_EngineComponent`)) (`/Game/Core/Vehicles/PDA_CameraSettings.MaxSpeed` _camerasettings)) 100.0)))

(event `Tick3rdPersonCameraRotation`
  (bind (_3rdpersoncamerarotation_roll _3rdpersoncamerarotation_pitch _3rdpersoncamerarotation_yaw) (`KismetMathLibrary.BreakRotator` (`self.3rdPersonCameraRotation`)))
  (bind _currentspeed (`/Game/Core/Vehicles/BP_EngineComponent.CurrentSpeed` (`self.BP_EngineComponent`)))
  (if (< (`KismetMathLibrary.Abs` _currentspeed) (`/Game/Core/Vehicles/PDA_CameraSettings.IdleSpeed` (`self.CameraSettings`)))
    (if (<= (`self.IdleCameraTimer`) 0.0)
      (set `self.3rdPersonCameraRotation` (`KismetMathLibrary.MakeRotator` 0.0 0.0 (+ _3rdpersoncamerarotation_yaw (`/Game/Core/Vehicles/PDA_CameraSettings.IdleRotationSpeed` (`self.CameraSettings`)))))
      (else
        (set `self.IdleCameraTimer` (`KismetMathLibrary.FInterpTo_Constant` (`self.IdleCameraTimer`) 0.0 (`GameplayStatics.GetWorldDeltaSeconds`) 1.0))))
    (else
      (set `self.IdleCameraTimer` (`/Game/Core/Vehicles/PDA_CameraSettings.IdleTime` (`self.CameraSettings`)))
      (set `self.3rdPersonCameraRotation` (select `bool` (xor (>= (`KismetMathLibrary.SignOfFloat` _currentspeed) 0.0) (`self.LookBehind`)) :`false` (struct :`Pitch` -50.0 :`Yaw` -180.0) :!type "Rotator Structure"))))
  (`SceneComponent.K2_SetRelativeRotation` (`self.3rdPersonArm`) (`KismetMathLibrary.ComposeRotators` (`self.3rdPersonCameraRotation`) (`self.CameraAngleOffset`)) false false))

(event `StartCameraShake`
  (`CameraShakeSourceComponent.StartCameraShake` :`self` (`self.CameraShakeSource`) :`InCameraShake` "/Game/Core/Data/NewCameraShakeBase.NewCameraShakeBase_C"))

(event `TickCameraAngle`
  (bind _camerasettings (`self.CameraSettings`))
  (bind _returnvalue (`KismetMathLibrary.GetRuntimeFloatCurveValue` (`/Game/Core/Vehicles/PDA_CameraSettings.CameraAnglesOverSpeed` _camerasettings) (/ (`/Game/Core/Vehicles/BP_EngineComponent.CurrentSpeed` (`self.BP_EngineComponent`)) (`/Game/Core/Vehicles/PDA_CameraSettings.MaxSpeed` _camerasettings)) 20.0))
  (set `self.CameraAngleOffset` (`KismetMathLibrary.MakeRotator` 0.0 (* _returnvalue -1.0)))
  (`SceneComponent.K2_SetRelativeRotation` (`self.3rdPersonCamera`) (`KismetMathLibrary.MakeRotator` 0.0 (* _returnvalue (`/Game/Core/Vehicles/PDA_CameraSettings.CameraAngleModifier` _camerasettings))) false false))

(event `Tick1stPersonCameraRotation`
  (bind (_1stpersoncamerarotation_roll _1stpersoncamerarotation_pitch _1stpersoncamerarotation_yaw) (`KismetMathLibrary.BreakRotator` (`self.1stPersonCameraRotation`)))
  (bind (_returnvalue_x _returnvalue_y) (`KismetMathLibrary.BreakVector2D` (* (`|GetInputActionValue`) (`self.LookSensitivity`))))
  (if (and (`self.HasInteriorCamera`) (`|EnumEquality` (`self.CurrentCamera`) "NewEnumerator1"))
    (bind _output_get (set `self.1stPersonCameraRotation` (`KismetMathLibrary.MakeRotator` _1stpersoncamerarotation_roll (`KismetMathLibrary.FClamp` (+ _1stpersoncamerarotation_pitch _returnvalue_y) -40.0 30.0) (`KismetMathLibrary.FClamp` (+ _1stpersoncamerarotation_yaw _returnvalue_x) -110.0 110.0))))
    (`SceneComponent.K2_SetRelativeRotation` (`self.1stPersonArm`) _output_get false false)
    (goto _label :!via `Reset`)
    (else
      (`/Engine/EditorBlueprintResources/StandardMacros.DoOnce` false :!label _label
        (:`Completed`
          (set `self.1stPersonCameraRotation` (struct)))))))

(event `BeginPlayAudio`
  (bind _fmodaudio (`self.FMODAudio`))
  (bind _asgi_global_game_instance (cast `/Game/Core/GI_GlobalGameInstance` (`GameplayStatics.GetGameInstance`)))
  (`FMODAudioComponent.SetParameter` _fmodaudio "Wind Volume" (* (`self.WindSFXVolume`) (`/Game/Core/GI_GlobalGameInstance.EffectsVolume` _asgi_global_game_instance)))
  (`FMODAudioComponent.SetParameter` _fmodaudio "Aggressiveness SFX" (`self.EngineSFXAggressiveness`)))

(event `TickAudio`
  (bind _bp_enginecomponent (`self.BP_EngineComponent`))
  (bind _bp_enginecomponent_2 (`self.BP_EngineComponent`))
  (bind _fmodaudio (`self.FMODAudio`))
  (bind _currentrpmratio (`/Game/Core/Vehicles/BP_EngineComponent.CurrentRPMRatio` _bp_enginecomponent_2))
  (bind _currentgear (`/Game/Core/Vehicles/BP_EngineComponent.CurrentGear` _bp_enginecomponent_2))
  (bind _output_get (set `self.CurrentThrottle` (`KismetMathLibrary.FInterpTo` (`self.CurrentThrottle`) (`KismetMathLibrary.FClamp` (* (`self.ThrottleInput`) (`/Game/Core/Vehicles/BP_EngineComponent.CurrentLoadMultiplierWhileGearShifting` _bp_enginecomponent) (`KismetMathLibrary.Abs` (`/Game/Core/Vehicles/BP_EngineComponent.CurrentSpeed` _bp_enginecomponent)))) (`GameplayStatics.GetWorldDeltaSeconds`) 10.0)))
  (`FMODAudioComponent.SetParameter` _fmodaudio "Engine Load" _output_get)
  (bind _output_get_2 (set `self.CurrentRPMRatio` (`KismetMathLibrary.SelectFloat` (`KismetMathLibrary.SelectFloat` (`KismetMathLibrary.FClamp` _currentrpmratio 0.0 0.95) _currentrpmratio (or (== (`KismetArrayLibrary.Array_LastIndex` (`/Game/Core/Vehicles/PDA_EngineSettings.GearRatios` (`/Game/Core/Vehicles/BP_EngineComponent.EngineSettings` _bp_enginecomponent_2))) _currentgear) (== _currentgear -1))) (`KismetMathLibrary.FInterpTo` (`self.CurrentRPMRatio`) _output_get (`GameplayStatics.GetWorldDeltaSeconds`) 1.0) (`/Game/Core/Vehicles/BP_EngineComponent.Grounded` (`self.BP_EngineComponent`)))))
  (`FMODAudioComponent.SetParameter` _fmodaudio "Engine RPM" (* _output_get_2 7000.0))
  (bind _returnvalue (`PrimitiveComponent.GetPhysicsLinearVelocity` (`self.Body`) "None"))
  (`FMODAudioComponent.SetParameter` _fmodaudio "Current Speed" (* (`KismetMathLibrary.VSize` _returnvalue) 0.036)))

(event `OnNitroxActivated`
  (bind _bp_enginecomponent (`self.BP_EngineComponent`))
  (`self.ActivateNitroxParticles`)
  (set `/Game/Core/Vehicles/BP_EngineComponent.NitroxActive` true _bp_enginecomponent)
  (set `self.CurrentNitroxDuration` (`/Game/Core/Vehicles/PDA_NitroxSettings.NitroxDuration` (`/Game/Core/Vehicles/BP_EngineComponent.NitroxSettings` _bp_enginecomponent)))
  (`GameplayStatics.PlaySoundAtLocation` "/Game/Effects/Audio/NitroxBoost.NitroxBoost" (`SceneComponent.K2_GetComponentLocation` (`self.Body`)) (struct) 1.0 1.0 0.0 null null null null))

(event `TickNitroxCooldown`
  (set `self.CurrentNitroxCooldown` (`KismetMathLibrary.FInterpTo_Constant` (`self.CurrentNitroxCooldown`) 0.0 (`GameplayStatics.GetWorldDeltaSeconds`) 1.0))
  (`/Game/Core/Engine/BPFL_DebugFunctions.PrintMessage` (`KismetStringLibrary.Concat_StrStr` "Nitrox: " (`KismetStringLibrary.Conv_IntToString` (`KismetMathLibrary.Round` (`self.CurrentNitrox`))) " Cooldown: " (`KismetStringLibrary.Conv_IntToString` (`KismetMathLibrary.Round` (`self.CurrentNitroxCooldown`))) " Duration: " (`KismetStringLibrary.Conv_IntToString` (`KismetMathLibrary.Round` (`self.CurrentNitroxDuration`)))) "NewEnumerator0" true))

(event `EnhancedInput|/Game/Core/Inputs/IA_Nitrox`
  (params (ActionValue :type Boolean) (ElapsedSeconds :type "Float (double-precision)") (TriggeredSeconds :type "Float (double-precision)") (InputAction :type "InputAction Object Reference" :default "/Game/Core/Inputs/IA_Nitrox.IA_Nitrox"))
  (bind _body (`self.Body`))
  (bind _nitroxsettings (`/Game/Core/Vehicles/BP_EngineComponent.NitroxSettings` (`self.BP_EngineComponent`)))
  (:`Triggered`
    (if (and (<= (`self.CurrentNitroxCooldown`) 0.0) (> (`self.CurrentNitrox`) 0.0))
      (`/Engine/EditorBlueprintResources/StandardMacros.DoOnce` false :!label _label
        (:`Completed`
          (`|ExecutionSequence`
            (:`then_0`
              (`self.OnNitroxActivated`))
            (:`then_1`
              (goto _label_3 :!via `Open`))
            (:`then_2`
              (goto _label_2 :!via `Reset`)))))))
  (:`Completed`
    (`|ExecutionSequence`
      (:`then_0`
        (goto _label :!via `Reset`))
      (:`then_1`
        (`/Engine/EditorBlueprintResources/StandardMacros.DoOnce` false :!label _label_2
          (:`Completed`
            (set `self.CurrentNitroxCooldown` (* (`/Game/Core/Vehicles/PDA_NitroxSettings.NitroxCooldown` _nitroxsettings) (`KismetMathLibrary.FClamp` (`KismetMathLibrary.MultiplyMultiply_FloatFloat` (- 1.0 (/ (`self.CurrentNitroxDuration`) (`/Game/Core/Vehicles/PDA_NitroxSettings.NitroxDuration` _nitroxsettings))) (`/Game/Core/Vehicles/PDA_NitroxSettings.NitroxCooldownExponent` _nitroxsettings)) (`/Game/Core/Vehicles/PDA_NitroxSettings.MinimumNitroxCooldownRatio` _nitroxsettings))))
            (`self.DeactivateNitroxParticles`)
            (set `/Game/Core/Vehicles/BP_EngineComponent.NitroxActive` false (`self.BP_EngineComponent`))
            (goto _label_3 :!via `Close`)))))))

(event `TickNitrox`
  (bind _body (`self.Body`))
  (`/Engine/EditorBlueprintResources/StandardMacros.Gate` true :!label _label_3
    (:`Exit`
      (if (`/Game/Core/Vehicles/BP_EngineComponent.Grounded` (`self.BP_EngineComponent`))
        (`|ExecutionSequence`
          (:`then_0`
            (`PrimitiveComponent.AddForce` _body (* (`SceneComponent.GetForwardVector` _body) (`/Game/Core/Vehicles/PDA_NitroxSettings.NitroxBoostForce` (`/Game/Core/Vehicles/BP_EngineComponent.NitroxSettings` (`self.BP_EngineComponent`))) (`self.ThrottleInput`)) "None" false))
          (:`then_1`
            (bind _output_get (set `self.CurrentNitrox` (`KismetMathLibrary.FInterpTo_Constant` (`self.CurrentNitrox`) 0.0 (`GameplayStatics.GetWorldDeltaSeconds`) 1.0)))
            (if (<= _output_get 0.0)
              (`self.ForceCompleteNitrox` :!label _label_4)))
          (:`then_2`
            (bind _output_get_2 (set `self.CurrentNitroxDuration` (`KismetMathLibrary.FInterpTo_Constant` (`self.CurrentNitroxDuration`) 0.0 (`GameplayStatics.GetWorldDeltaSeconds`) 1.0)))
            (if (<= _output_get_2 0.0)
              (goto _label_4)))
          (:`then_3`
            (if (`/Game/Core/Vehicles/BP_EngineComponent.Grounded` (`self.BP_EngineComponent`)) :!label _label_5
              (`|ExecutionSequence`
                (:`then_0`
                  (`/Engine/EditorBlueprintResources/StandardMacros.DoOnce` true :!label _label_6
                    (:`Completed`
                      (`self.ActivateNitroxParticles`))))
                (:`then_1`
                  (goto _label_7 :!via `Reset`)))
              (else
                (`|ExecutionSequence`
                  (:`then_0`
                    (`/Engine/EditorBlueprintResources/StandardMacros.DoOnce` false :!label _label_7
                      (:`Completed`
                        (`self.DeactivateNitroxParticles`))))
                  (:`then_1`
                    (goto _label_6 :!via `Reset`)))))))
        (else
          (goto _label_5))))))

(event `ForceCompleteNitrox`
  (goto _label_2))

(event `BeginPlaySetupNitrox`
  (set `self.CurrentNitrox` (`/Game/Core/Vehicles/PDA_NitroxSettings.NitroxFuelAmount` (`/Game/Core/Vehicles/BP_EngineComponent.NitroxSettings` (`self.BP_EngineComponent`))))
  (`self.SetNitroxMaterials`))

(event `TickCollectInputs`
  (set `self.ThrottleInput` (`|GetInputActionValue`))
  (set `self.SteeringInput` (`|GetInputActionValue`)))

(event `EnhancedInput|/Game/Core/Inputs/IA_LookBehind`
  (params (ActionValue :type "Vector2D Structure") (ElapsedSeconds :type "Float (double-precision)") (TriggeredSeconds :type "Float (double-precision)") (InputAction :type "InputAction Object Reference" :default "/Game/Core/Inputs/IA_LookBehind.IA_LookBehind"))
  (:`Triggered`
    (set `self.LookBehind` true :!label _label)
    (bind (_direction _speed) (`Timeline|Timeline` :!label _label_2)
      (:`Update`
        (set `SpringArmComponent.CameraRotationLagSpeed` _speed (`self.3rdPersonArm`)))))
  (:`Started`
    (goto _label))
  (:`Canceled`
    (set `self.LookBehind` false :!label _label_3)
    (goto _label_2 :!via `Reverse`))
  (:`Completed`
    (goto _label_3)))

(event `EnhancedInput|/Game/Core/Inputs/IA_GearShift`
  (params (ActionValue :type "Float (double-precision)") (ElapsedSeconds :type "Float (double-precision)") (TriggeredSeconds :type "Float (double-precision)") (InputAction :type "InputAction Object Reference" :default "/Game/Core/Inputs/IA_GearShift.IA_GearShift"))
  (bind _bp_enginecomponent (`self.BP_EngineComponent`))
  (:`Started`
    (if (> ActionValue 0.0)
      (`/Game/Core/Vehicles/BP_EngineComponent.GearChangeUp` _bp_enginecomponent)
      (elif (< ActionValue 0.0)
        (`/Game/Core/Vehicles/BP_EngineComponent.GearChangeDown` _bp_enginecomponent)))))

(event `BeginPlayManualGearShift`
  (bind _asgi_global_game_instance (cast `/Game/Core/GI_GlobalGameInstance` (`GameplayStatics.GetGameInstance`)))
  (set `/Game/Core/Vehicles/BP_EngineComponent.ManualGearShifting` (`/Game/Core/GI_GlobalGameInstance.ManualGearShifting` _asgi_global_game_instance) (`self.BP_EngineComponent`)))

(event `EnhancedInput|/Game/Core/Inputs/IA_SwitchCamera`
  (params (ActionValue :type Boolean) (ElapsedSeconds :type "Float (double-precision)") (TriggeredSeconds :type "Float (double-precision)") (InputAction :type "InputAction Object Reference" :default "/Game/Core/Inputs/IA_SwitchCamera.IA_SwitchCamera"))
  (:`Started`
    (switch `/Game/Core/Engine/E_CameraSelection` (`self.CurrentCamera`)
      (:`NewEnumerator0`
        (set `self.CurrentCamera` "NewEnumerator2"))
      (:`NewEnumerator2`
        (if (`self.HasInteriorCamera`)
          (set `self.CurrentCamera` "NewEnumerator1")
          (else
            (set `self.CurrentCamera` "NewEnumerator0"))))
      (:`NewEnumerator1`
        (set `self.CurrentCamera` "NewEnumerator0")))
    (`self.SwitchCamera`)))

(event `TickUpdateDrifting`
  (bind _body (`self.Body`))
  (bind _returnvalue (`PrimitiveComponent.GetPhysicsLinearVelocity` _body "None"))
  (bind _returnvalue_2 (`KismetMathLibrary.Normal` (`KismetMathLibrary.ProjectVectorOnToPlane` _returnvalue (`SceneComponent.GetUpVector` _body))))
  (bind _returnvalue_3 (`KismetMathLibrary.Abs` (`KismetMathLibrary.Dot_VectorVector` (`SceneComponent.GetForwardVector` _body) _returnvalue_2)))
  (bind _output_get (set `self.CurrentSlip` _returnvalue_3))
  (`|ExecutionSequence`
    (:`then_0`
      (for _array_element (`/Game/Core/Vehicles/BP_EngineComponent.WheelRefs` (`self.BP_EngineComponent`))
        (if (and (< _output_get (`self.DriftingTreshold`)) (`/Game/Core/Vehicles/BP_WheelComponent.Grounded` _array_element))
          (bind _drifting (`/Game/Core/Vehicles/BP_WheelComponent.Drifting` _array_element))
          (if (not _drifting)
            (`self.ActivateDriftingParticles` _array_element)
            (set `/Game/Core/Vehicles/BP_WheelComponent.Drifting` true _array_element))
          (elif _drifting
            (`self.DeactivateDriftingParticles` _array_element)
            (set `/Game/Core/Vehicles/BP_WheelComponent.Drifting` false _array_element)))))
    (:`then_1`
      (`self.UpdateDriftingParticles` (`/Game/Core/Vehicles/BP_WheelComponent.GroundNormal` (`|GetArrayItem` (`/Game/Core/Vehicles/BP_EngineComponent.WheelRefs` (`self.BP_EngineComponent`)))) _returnvalue_2 _returnvalue_3))))

(fn `ActivateDriftingParticles`
  (params (WheelRef :type "/Game/Core/Vehicles/BP_WheelComponent Object Reference")))

(fn `ActivateNitroxParticles`)

(fn `DeactivateDriftingParticles`
  (params (WheelRef :type "/Game/Core/Vehicles/BP_WheelComponent Object Reference")))

(fn `DeactivateNitroxParticles`)

(fn `SetNitroxMaterials`)

(fn `SwitchCamera`
  (bind _hoodcamera (`self.HoodCamera`))
  (bind _1stpersoncamera (`self.1stPersonCamera`))
  (bind _fmodaudio (`self.FMODAudio`))
  (switch `/Game/Core/Engine/E_CameraSelection` (`self.CurrentCamera`)
    (:`NewEnumerator0`
      (`ActorComponent.Activate` (`self.3rdPersonCamera`) false)
      (`ActorComponent.Activate` (`self.NS_3rdPersonSpeedLines`) false)
      (`FMODAudioComponent.SetParameter` _fmodaudio "Exterior-Interior" 0.0)
      (`|ExecutionSequence`
        (:`then_0`
          (`ActorComponent.Deactivate` _hoodcamera :!label _label)
          (`ActorComponent.Deactivate` (`self.NS_HoodSpeedParticle`)))
        (:`then_1`
          (`ActorComponent.Deactivate` _1stpersoncamera :!label _label_2))))
    (:`NewEnumerator2`
      (`ActorComponent.Activate` _hoodcamera false)
      (`ActorComponent.Activate` (`self.NS_HoodSpeedParticle`) false)
      (`FMODAudioComponent.SetParameter` _fmodaudio "Exterior-Interior" 0.0)
      (`|ExecutionSequence`
        (:`then_0`
          (`ActorComponent.Deactivate` (`self.NS_3rdPersonSpeedLines`) :!label _label_3)
          (`ActorComponent.Deactivate` (`self.3rdPersonCamera`)))
        (:`then_1`
          (goto _label_2))))
    (:`NewEnumerator1`
      (`ActorComponent.Activate` _1stpersoncamera false)
      (`FMODAudioComponent.SetParameter` _fmodaudio "Exterior-Interior" 1.0)
      (`|ExecutionSequence`
        (:`then_0`
          (goto _label_3))
        (:`then_1`
          (goto _label))))))

(fn `UpdateDriftingParticles`
  (params (GroundNormal :type "Vector Structure") (VelocityNormalized :type "Vector Structure") (CurrentSlip :type "Float (double-precision)")))

(fn `UpdateNitroxUpDirection`)

(fn `UserConstructionScript`)