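; Vehicle engine component that drives the owner's physics root body and its BP_WheelComponents.
; Each tick it measures forward speed, applies custom gravity, drag and grounded downforce, then derives gear and a smoothed RPM ratio from speed.
; Throttle input combines RPM curve, turbo, nitrox and gear multipliers into per-wheel acceleration or braking, while steering adds automatic countersteer and airborne angular damping.
; Automatic or manual shifts dip power, reset turbo and play shift and backfire sounds.
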(event `self.ReceiveBeginPlay`
  (`self.GetPhysicsBody`)
  (`self.GetWheels`))

(event `self.ReceiveTick`
  (params (DeltaSeconds :type "Float (single-precision)"))
  (`self.TickUpdateSpeed`)
  (`self.TickGravity`)
  (`self.TickDrag`)
  (`self.TickDownForce`)
  (`self.TickGear`)
  (`self.TickGearShiftValues`)
  (`self.TickCurrentRPM`))

(event `GetPhysicsBody`
  (bind _asprimitive_component (cast `PrimitiveComponent` (`Actor.RootComponent` (`self.GetOwner`)))
    (:`then`
      (if (`SceneComponent.IsSimulatingPhysics` _asprimitive_component "None")
        (set `self.PhysicsBodyRef` _asprimitive_component)
        (else
          (`/Game/Core/Engine/BPFL_DebugFunctions.PrintMessage` "Owning root component is not physics enabled" "NewEnumerator1")
          (`/Game/Core/Engine/BPFL_DebugFunctions.PrintMessage` "Enabling physics on root component..." "NewEnumerator2")
          (`PrimitiveComponent.SetSimulatePhysics` _asprimitive_component true)
          (set `self.PhysicsBodyRef` _asprimitive_component))))
    (:`CastFailed`
      (`/Game/Core/Engine/BPFL_DebugFunctions.PrintMessage` "Owning root component is not physics compatible" "NewEnumerator1"))))

(event `GetWheels`
  (bind _returnvalue (`Actor.K2_GetComponentsByClass` (`self.GetOwner`) "/Game/Core/Vehicles/BP_WheelComponent.BP_WheelComponent_C"))
  (if (> (`KismetArrayLibrary.Array_Length` _returnvalue) 0)
    (bind _output_get (set `self.WheelRefs` _returnvalue))
    (for _array_element _output_get
      (set `self.Differential` (+ (`/Game/Core/Vehicles/BP_WheelComponent.ThrottleModifier` _array_element) (`self.Differential`))))
    (else
      (`/Game/Core/Engine/BPFL_DebugFunctions.PrintMessage` "Owning actor has no wheels" "NewEnumerator1"))))

(event `InputSteering`
  (params (Steering :type "Float (double-precision)"))
  (bind _physicsbodyref (`self.PhysicsBodyRef`))
  (bind _physicsbodyref_2 (`self.PhysicsBodyRef`))
  (bind _returnvalue (`SceneComponent.GetUpVector` _physicsbodyref))
  (bind (_returnvalue_x _returnvalue_y _returnvalue_z) (`KismetMathLibrary.BreakVector` (`KismetMathLibrary.ProjectVectorOnToVector` (`PrimitiveComponent.GetPhysicsAngularVelocityInDegrees` _physicsbodyref "None") _returnvalue)))
  (set `self.Grounded` false)
  (for _array_element (`self.WheelRefs`)
    (if (!= (`/Game/Core/Vehicles/BP_WheelComponent.SteeringModifier` _array_element) 0.0)
      (`/Game/Core/Vehicles/BP_WheelComponent.TickSteering` _array_element (`KismetMathLibrary.SelectFloat` (`KismetMathLibrary.FClamp` (* (/ _returnvalue_z -100.0) (`KismetMathLibrary.SignOfFloat` (`KismetMathLibrary.Dot_VectorVector` _returnvalue (`KismetMathLibrary.Vector_Up`))) (`KismetMathLibrary.SignOfFloat` (`self.CurrentSpeed`)) (`self.SteeringCompensation`)) -0.5 0.5) Steering (== Steering 0.0))))
    (if (`/Game/Core/Vehicles/BP_WheelComponent.Grounded` _array_element)
      (set `self.Grounded` true)))
  (if (`self.Grounded`)
    (`PrimitiveComponent.SetAngularDamping` _physicsbodyref_2 0.0)
    (else
      (`PrimitiveComponent.SetAngularDamping` _physicsbodyref_2 (`/Game/Core/Vehicles/PDA_EngineSettings.AirborneAngularDamping` (`self.EngineSettings`))))))

(event `InputThrottle`
  (params (Throttle :type "Float (double-precision)"))
  (bind _returnvalue (`KismetMathLibrary.Abs` Throttle))
  (bind _enginesettings (`self.EngineSettings`))
  (bind _turbosettings (`self.TurboSettings`))
  (bind _currentturbostrength (`self.CurrentTurboStrength`))
  (bind _returnvalue_2 (> _currentturbostrength _returnvalue))
  (if (`/Game/Core/Vehicles/PDA_TurboSettings.HasTurbo` _turbosettings)
    (if _returnvalue_2
      (`|ExecutionSequence`
        (:`then_0`
          (`/Engine/EditorBlueprintResources/StandardMacros.DoOnce` false :!label _label
            (:`Completed`
              (if (`KismetMathLibrary.RandomBoolWithWeight` (`/Game/Core/Vehicles/PDA_TurboSettings.NitroWhistleChance` (`self.TurboSettings`)))
                (`GameplayStatics.PlaySoundAtLocation` "/Game/Effects/Audio/Exhausts/TurboWhistle.TurboWhistle" (`Actor.K2_GetActorLocation` (`self.GetOwner`)) (struct) 1.0 1.0 0.0 null null null null)))))
        (:`then_1`
          (set `self.CurrentTurboStrength` (`KismetMathLibrary.FInterpTo_Constant` _currentturbostrength (`KismetMathLibrary.SelectFloat` (`self.CurrentRPMRatio`) _returnvalue (`/Game/Core/Vehicles/PDA_TurboSettings.IsSupercharger` _turbosettings)) (`GameplayStatics.GetWorldDeltaSeconds`) (/ 1.0 (`KismetMathLibrary.SelectFloat` (`/Game/Core/Vehicles/PDA_TurboSettings.DurationToEmptyTurbo` _turbosettings) (`/Game/Core/Vehicles/PDA_TurboSettings.DurationToEmptyTurbo` _turbosettings) _returnvalue_2))) :!label _label_2)
          (bind _output_get (set `self.CurrentThrottle` Throttle :!label _label_3))
          (if (`self.Grounded`)
            (for _array_element (`self.WheelRefs`)
              (if (!= (`self.CurrentThrottle`) 0.0)
                (bind _throttlemodifier (`/Game/Core/Vehicles/BP_WheelComponent.ThrottleModifier` _array_element))
                (if (!= _throttlemodifier 0.0)
                  (bind _returnvalue_3 (/ (`KismetMathLibrary.SelectFloat` (* (`KismetMathLibrary.GetRuntimeFloatCurveValue` (`/Game/Core/Vehicles/PDA_EngineSettings.AccelerationOverRPMRatio` _enginesettings) (`self.CurrentRPMRatio`) 1.0) (* (`/Game/Core/Vehicles/PDA_EngineSettings.MaxAcceleration` _enginesettings) (`KismetMathLibrary.Lerp` 1.0 (`/Game/Core/Vehicles/PDA_TurboSettings.TurboStrength` (`self.TurboSettings`)) (`self.CurrentTurboStrength`)) (`KismetMathLibrary.SelectFloat` (`KismetMathLibrary.FClamp` Throttle) (`KismetMathLibrary.FClamp` Throttle -1.0 0.0) (> (`self.CurrentGear`) 0)))) (* (`/Game/Core/Vehicles/PDA_EngineSettings.BrakingForce` (`self.EngineSettings`)) Throttle) (>= (`KismetMathLibrary.SignOfFloat` (* _output_get (`self.CurrentSpeed`))) 0.0)) (`self.Differential`)))
                  (`/Game/Core/Vehicles/BP_WheelComponent.TickAcceleration` _array_element (* _throttlemodifier (`KismetMathLibrary.SelectFloat` (* _returnvalue_3 (`/Game/Core/Vehicles/PDA_NitroxSettings.NitroxAccelerationBoost` (`self.NitroxSettings`))) _returnvalue_3 (`self.NitroxActive`)) (`self.CurrentLoadMultiplierWhileGearShifting`) (`|GetArrayItem` (`/Game/Core/Vehicles/PDA_EngineSettings.GearPowerMultilpiers` (`self.EngineSettings`)) (- (`KismetMathLibrary.Abs_Int` (`self.CurrentGear`)) 1)))))
                (else
                  (`/Game/Core/Vehicles/BP_WheelComponent.TickLongitunalGrip` _array_element)))))))
      (else
        (`|ExecutionSequence`
          (:`then_0`
            (goto _label :!via `Reset`))
          (:`then_1`
            (goto _label_2)))))
    (else
      (goto _label_3))))

(event `TickUpdateSpeed`
  (bind _physicsbodyref (`self.PhysicsBodyRef`)
    (:`then`
      (bind _returnvalue (`PrimitiveComponent.GetPhysicsLinearVelocity` _physicsbodyref "None"))
      (bind _returnvalue_2 (`KismetMathLibrary.ProjectVectorOnToPlane` _returnvalue (`SceneComponent.GetUpVector` _physicsbodyref)))
      (bind _returnvalue_3 (`SceneComponent.GetForwardVector` _physicsbodyref))
      (bind _returnvalue_4 (`KismetMathLibrary.Dot_VectorVector` _returnvalue_2 _returnvalue_3))
      (set `self.CurrentSpeed` _returnvalue_4)
      (bind _returnvalue_5 (`KismetMathLibrary.Abs` (`KismetMathLibrary.Dot_VectorVector` _returnvalue_3 (`KismetMathLibrary.Normal` _returnvalue_2))))
      (set `self.CurrentSlip` _returnvalue_5)
      (`/Game/Core/Engine/BPFL_DebugFunctions.PrintMessage` (`KismetStringLibrary.Concat_StrStr` "Speed: " (`KismetStringLibrary.Conv_IntToString` (`KismetMathLibrary.Round` _returnvalue_4)) "cm/s or " (`KismetStringLibrary.Conv_IntToString` (`KismetMathLibrary.Round` (* _returnvalue_4 0.036))) "kph") "NewEnumerator0" true)
      (`/Game/Core/Engine/BPFL_DebugFunctions.PrintMessage` (`KismetStringLibrary.Concat_StrStr` "Slip Ratio: " (`KismetStringLibrary.Conv_DoubleToString` _returnvalue_5)) "NewEnumerator0" true))
    (:`else`)))

(event `TickDownForce`
  (bind _enginesettings (`self.EngineSettings`))
  (bind _physicsbodyref (`self.PhysicsBodyRef`))
  (if (`self.Grounded`)
    (`PrimitiveComponent.AddForce` _physicsbodyref (* (`SceneComponent.GetUpVector` _physicsbodyref) (`KismetMathLibrary.FClamp` (* (`self.CurrentSpeed`) (`/Game/Core/Vehicles/PDA_EngineSettings.DownForceStrength` _enginesettings)) 0.0 (`/Game/Core/Vehicles/PDA_EngineSettings.MaxDownForce` _enginesettings)) -1.0) "None" false)))

(event `TickGravity`
  (`PrimitiveComponent.AddForce` (`self.PhysicsBodyRef`) (* (`KismetMathLibrary.Vector_Up`) (`/Game/Core/Engine/BPFL_GlobalConstants.GlobalGravity`) (`self.GravityModifier`) -1) "None" true))

(event `TickDrag`
  (bind _physicsbodyref (`self.PhysicsBodyRef`))
  (`PrimitiveComponent.AddForce` _physicsbodyref (* (`SceneComponent.GetForwardVector` _physicsbodyref) (* (`self.CurrentSpeed`) (`/Game/Core/Vehicles/PDA_EngineSettings.Drag` (`self.EngineSettings`)) -1.0)) "None" false))

(event `TickGear`
  (bind _enginesettings (`self.EngineSettings`))
  (bind _gearratios (`/Game/Core/Vehicles/PDA_EngineSettings.GearRatios` _enginesettings))
  (bind _returnvalue (/ (`self.CurrentSpeed`) (`/Game/Core/Vehicles/PDA_EngineSettings.MaxSpeed` _enginesettings)))
  (for _index (range (`KismetArrayLibrary.Array_LastIndex` _gearratios))
    (if (and (> _returnvalue (`|GetArrayItem` _gearratios _index)) (< _returnvalue (`|GetArrayItem` _gearratios (+ _index 1))))
      (`self.ChangeGear` (+ _index 1))
      (break)
      (elif (< _returnvalue 0.0)
        (`self.ChangeGear` -1)
        (break)))))

(event `TickGearShiftValues`
  (set `self.CurrentLoadMultiplierWhileGearShifting` (`KismetMathLibrary.FInterpTo_Constant` (`self.CurrentLoadMultiplierWhileGearShifting`) 1.0 (`GameplayStatics.GetWorldDeltaSeconds`) (/ 1.0 (`/Game/Core/Vehicles/PDA_EngineSettings.GearShiftDuration` (`self.EngineSettings`)))))
  (set `self.CurrentGearShiftCooldown` (`KismetMathLibrary.FInterpTo_Constant` (`self.CurrentGearShiftCooldown`) 0.0 (`GameplayStatics.GetWorldDeltaSeconds`) 1.0))
  (`/Game/Core/Engine/BPFL_DebugFunctions.PrintMessage` (`KismetStringLibrary.BuildString_Int` "" "Current Gear: " (`self.CurrentGear`) (`KismetStringLibrary.BuildString_Int` " \n" "Recommended Gear: " (`self.RecommendedGear`))) "NewEnumerator0" true))

(event `TickCurrentRPM`
  (bind _currentgear (`self.CurrentGear`))
  (bind _currentgear_2 (`self.CurrentGear`))
  (bind _enginesettings (`self.EngineSettings`))
  (bind _returnvalue (< _currentgear_2 0))
  (bind _gearshiftforgiveness (`/Game/Core/Vehicles/PDA_EngineSettings.GearShiftForgiveness` _enginesettings))
  (bind _gearratios (`/Game/Core/Vehicles/PDA_EngineSettings.GearRatios` _enginesettings))
  (bind _returnvalue_2 (* (`|GetArrayItem` _gearratios (`KismetMathLibrary.SelectInt` 0 (- _currentgear_2 1) _returnvalue)) (- 1.0 _gearshiftforgiveness)))
  (bind _returnvalue_3 (`KismetMathLibrary.FInterpTo` (`self.CurrentRPMRatio`) (* (`KismetMathLibrary.SignOfInteger` (`self.CurrentGear`)) (/ (- (/ (`self.CurrentSpeed`) (`/Game/Core/Vehicles/PDA_EngineSettings.MaxSpeed` _enginesettings)) _returnvalue_2) (* (- (`|GetArrayItem` _gearratios (`KismetMathLibrary.SelectInt` 1 _currentgear_2 _returnvalue)) _returnvalue_2) (+ 1.0 _gearshiftforgiveness)))) (`GameplayStatics.GetWorldDeltaSeconds`) 5.0))
  (bind _output_get (set `self.CurrentRPMRatio` (`KismetMathLibrary.SelectFloat` (`KismetMathLibrary.FClamp` _returnvalue_3 (`/Game/Core/Vehicles/PDA_EngineSettings.IdleRPMRatio` (`self.EngineSettings`)) 2.0) _returnvalue_3 (or (== _currentgear 1) (== _currentgear -1)))))
  (`/Game/Core/Engine/BPFL_DebugFunctions.PrintMessage` (`KismetStringLibrary.Conv_DoubleToString` _output_get) "NewEnumerator0" true))

(event `ChangeGear`
  (params (NewGear :type Integer))
  (bind _currentgear (`self.CurrentGear`))
  (bind _enginesettings (`self.EngineSettings`))
  (set `self.RecommendedGear` NewGear)
  (if (not (`self.ManualGearShifting`))
    (if (and (!= NewGear _currentgear) (<= (`self.CurrentGearShiftCooldown`) 0.0))
      (if (> NewGear _currentgear)
        (set `self.CurrentLoadMultiplierWhileGearShifting` (`/Game/Core/Vehicles/PDA_EngineSettings.LoadMultiplierWhileGearShifting` _enginesettings)))
      (set `self.CurrentGear` NewGear)
      (set `self.CurrentGearShiftCooldown` (`/Game/Core/Vehicles/PDA_EngineSettings.GearShiftCooldown` _enginesettings))
      (`self.OnGearChanged`))))

(event `GearChangeUp`
  (bind _currentgear (`self.CurrentGear`))
  (if (== _currentgear -1)
    (set `self.CurrentGear` 1)
    (set `self.CurrentLoadMultiplierWhileGearShifting` (`/Game/Core/Vehicles/PDA_EngineSettings.LoadMultiplierWhileGearShifting` (`self.EngineSettings`)) :!label _label)
    (`self.OnGearChanged`)
    (elif (< _currentgear (- (`KismetArrayLibrary.Array_Length` (`/Game/Core/Vehicles/PDA_EngineSettings.GearRatios` (`self.EngineSettings`))) 1))
      (`/Engine/EditorBlueprintResources/StandardMacros.IncrementInt` _currentgear
        (:`  `
          (goto _label))))))

(event `GearChangeDown`
  (bind _currentgear (`self.CurrentGear`))
  (if (== _currentgear 1)
    (set `self.CurrentGear` -1)
    (set `self.CurrentLoadMultiplierWhileGearShifting` (`/Game/Core/Vehicles/PDA_EngineSettings.LoadMultiplierWhileGearShifting` (`self.EngineSettings`)) :!label _label_2)
    (`self.OnGearChanged`)
    (elif (> _currentgear 1)
      (`/Engine/EditorBlueprintResources/StandardMacros.DecrementInt` _currentgear
        (:`  `
          (goto _label_2))))))

(event `OnGearChanged`
  (bind _turbosettings (`self.TurboSettings`))
  (bind _returnvalue (`SceneComponent.K2_GetComponentLocation` (`self.PhysicsBodyRef`)))
  (set `self.CurrentTurboStrength` 0.0)
  (`GameplayStatics.PlaySoundAtLocation` "/Game/Effects/Audio/Gearshifting/SC_GearShift.SC_GearShift" _returnvalue (struct) 0.5 1.0 0.0 "/Game/Effects/Audio/Gearshifting/GearShiftAttenuation.GearShiftAttenuation" null null null)
  (if (and (`KismetMathLibrary.RandomBoolWithWeight` (`/Game/Core/Vehicles/PDA_TurboSettings.BackfireChance` _turbosettings)) (>= (`self.CurrentRPMRatio`) (`/Game/Core/Vehicles/PDA_TurboSettings.BackfireCutoff` _turbosettings)))
    (`KismetSystemLibrary.Delay` 0.2)
    (`GameplayStatics.PlaySoundAtLocation` "/Game/Effects/Audio/Exhausts/SC_ExhaustBackfire.SC_ExhaustBackfire" _returnvalue (struct) 1.0 1.0 0.0 "/Game/Effects/Audio/Gearshifting/GearShiftAttenuation.GearShiftAttenuation" null null null)))