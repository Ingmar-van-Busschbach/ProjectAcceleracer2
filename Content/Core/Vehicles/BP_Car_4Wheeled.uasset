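; Four-wheeled car Blueprint that extends a parent vehicle class by implementing its nitrox and drifting particle hooks, calling the parent version first.
; Left and right nitrox effects toggle together and receive the nitrox material and their own up vectors.
; Drift effects toggle per wheel through that wheel's Niagara children.
; All four drift effects receive ground normal, velocity direction and slip as Niagara variables.
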(fn `ActivateDriftingParticles`
  (params (WheelRef :type "/Game/Core/Vehicles/BP_WheelComponent Object Reference"))
  (`parent.ActivateDriftingParticles` WheelRef)
  (for _array_element (`SceneComponent.GetChildrenComponents` WheelRef false)
    (bind _asniagara_particle_system_component (cast `NiagaraComponent` _array_element))
    (`ActorComponent.Activate` _asniagara_particle_system_component true)))

(fn `ActivateNitroxParticles`
  (`parent.ActivateNitroxParticles`)
  (`ActorComponent.Activate` (`self.NitroxParticleLeft`) true)
  (`ActorComponent.Activate` (`self.NitroxParticleRight`) true))

(fn `DeactivateDriftingParticles`
  (params (WheelRef :type "/Game/Core/Vehicles/BP_WheelComponent Object Reference"))
  (`parent.DeactivateDriftingParticles` WheelRef)
  (for _array_element (`SceneComponent.GetChildrenComponents` WheelRef false)
    (bind _asniagara_particle_system_component (cast `NiagaraComponent` _array_element))
    (`ActorComponent.Deactivate` _asniagara_particle_system_component)))

(fn `DeactivateNitroxParticles`
  (`parent.DeactivateNitroxParticles`)
  (`ActorComponent.Deactivate` (`self.NitroxParticleLeft`))
  (`ActorComponent.Deactivate` (`self.NitroxParticleRight`)))

(fn `SetNitroxMaterials`
  (`parent.SetNitroxMaterials`)
  (`NiagaraComponent.SetVariableMaterial` (`self.NitroxParticleLeft`) "Material" (`self.NitroxMaterial`))
  (`NiagaraComponent.SetVariableMaterial` (`self.NitroxParticleRight`) "Material" (`self.NitroxMaterial`)))

(fn `UpdateDriftingParticles`
  (params (GroundNormal :type "Vector Structure") (VelocityNormalized :type "Vector Structure") (CurrentSlip :type "Float (double-precision)"))
  (bind _driftparticlerearright (`self.DriftParticleRearRight`))
  (`parent.UpdateDriftingParticles` GroundNormal VelocityNormalized CurrentSlip)
  (`NiagaraComponent.SetVariableVec3` _driftparticlerearright "SpriteFacingDirectionNormal" GroundNormal)
  (`NiagaraComponent.SetVariableVec3` (`self.DriftParticleFrontRight`) "SpriteFacingDirectionNormal" GroundNormal)
  (`NiagaraComponent.SetVariableVec3` (`self.DriftParticleFrontLeft`) "SpriteFacingDirectionNormal" GroundNormal)
  (`NiagaraComponent.SetVariableVec3` (`self.DriftParticleRearLeft`) "SpriteFacingDirectionNormal" GroundNormal)
  (`NiagaraComponent.SetVariableVec3` _driftparticlerearright "SpriteAlignmentNormal" VelocityNormalized)
  (`NiagaraComponent.SetVariableVec3` (`self.DriftParticleFrontRight`) "SpriteAlignmentNormal" VelocityNormalized)
  (`NiagaraComponent.SetVariableVec3` (`self.DriftParticleFrontLeft`) "SpriteAlignmentNormal" VelocityNormalized)
  (`NiagaraComponent.SetVariableVec3` (`self.DriftParticleRearLeft`) "SpriteAlignmentNormal" VelocityNormalized)
  (`NiagaraComponent.SetVariableFloat` _driftparticlerearright "CurrentSlip" CurrentSlip)
  (`NiagaraComponent.SetVariableFloat` (`self.DriftParticleFrontRight`) "CurrentSlip" CurrentSlip)
  (`NiagaraComponent.SetVariableFloat` (`self.DriftParticleFrontLeft`) "CurrentSlip" CurrentSlip)
  (`NiagaraComponent.SetVariableFloat` (`self.DriftParticleRearLeft`) "CurrentSlip" CurrentSlip))

(fn `UpdateNitroxUpDirection`
  (bind _nitroxparticleleft (`self.NitroxParticleLeft`))
  (bind _nitroxparticleright (`self.NitroxParticleRight`))
  (`parent.UpdateNitroxUpDirection`)
  (`NiagaraComponent.SetVariableVec3` _nitroxparticleleft "UpDirection" (`SceneComponent.GetUpVector` _nitroxparticleleft))
  (`NiagaraComponent.SetVariableVec3` _nitroxparticleright "UpDirection" (`SceneComponent.GetUpVector` _nitroxparticleright)))

(fn `UserConstructionScript`
  (`parent.UserConstructionScript`))