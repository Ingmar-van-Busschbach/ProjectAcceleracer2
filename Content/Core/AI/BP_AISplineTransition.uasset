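; BP_AISplineTransition is a trigger that switches AI cars onto a new spline to follow.
; When a BP_CarBase with a BPC_AIControllerComponent overlaps its box, it records the car in AIArray and sets the component's SplineRef from a random SplineRoads entry.
; If that pick's spline is invalid, it tries a random SplineTools entry instead.
; Random is re-evaluated on assignment, so the assigned spline can differ from the validated one.
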(event `self.Box.OnComponentBeginOverlap`
  (params (OverlappedComponent :type "PrimitiveComponent Object Reference") (OtherActor :type "Actor Object Reference") (OtherComp :type "PrimitiveComponent Object Reference") (OtherBodyIndex :type Integer) (bFromSweep :type Boolean) (SweepResult :type "HitResult Structure (by ref)"))
  (bind _spline (`/Game/Core/Objects/SplineToolPro/Spline/SplineToolPro.Spline` (`KismetArrayLibrary.Array_Random` (`self.SplineTools`))))
  (bind _spline_2 (`/Game/Core/Objects/BP_SplineRoadTool.Spline` (`KismetArrayLibrary.Array_Random` (`self.SplineRoads`))))
  (bind _asbp_car_base (cast `/Game/Core/Vehicles/BP_CarBase` OtherActor))
  (bind _returnvalue (`self.GetComponentByClass` _asbp_car_base "/Game/Core/AI/BPC_AIControllerComponent.BPC_AIControllerComponent_C"))
  (`/Engine/EditorBlueprintResources/StandardMacros.IsValid` _returnvalue
    (:`Is Valid`
      (`KismetArrayLibrary.Array_Add` (`self.AIArray`) _asbp_car_base)
      (`/Engine/EditorBlueprintResources/StandardMacros.IsValid` _spline_2
        (:`Is Valid`
          (set `/Game/Core/AI/BPC_AIControllerComponent.SplineRef` _spline_2 _returnvalue))
        (:`Is Not Valid`
          (`/Engine/EditorBlueprintResources/StandardMacros.IsValid` _spline
            (:`Is Valid`
              (set `/Game/Core/AI/BPC_AIControllerComponent.SplineRef` _spline _returnvalue))))))))

(fn `UserConstructionScript`
  (`parent.UserConstructionScript`))