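; BP_AIBrakingZone is a box trigger that changes the top speed of AI-driven cars while they are inside it.
; On begin overlap, a BP_CarBase with a BPC_AIControllerComponent is added to AIArray and receives the zone's MaxSpeedMultiplier.
; On end overlap, cars found in AIArray have the multiplier reset to 1.0 but stay in the array.
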(event `self.Box.OnComponentBeginOverlap`
  (params (OverlappedComponent :type "PrimitiveComponent Object Reference") (OtherActor :type "Actor Object Reference") (OtherComp :type "PrimitiveComponent Object Reference") (OtherBodyIndex :type Integer) (bFromSweep :type Boolean) (SweepResult :type "HitResult Structure (by ref)"))
  (bind _asbp_car_base (cast `/Game/Core/Vehicles/BP_CarBase` OtherActor))
  (bind _returnvalue (`self.GetComponentByClass` _asbp_car_base "/Game/Core/AI/BPC_AIControllerComponent.BPC_AIControllerComponent_C"))
  (`/Engine/EditorBlueprintResources/StandardMacros.IsValid` _returnvalue
    (:`Is Valid`
      (`KismetArrayLibrary.Array_Add` (`self.AIArray`) _asbp_car_base)
      (set `/Game/Core/AI/BPC_AIControllerComponent.MaxSpeedMultiplier` (`self.MaxSpeedMultiplier`) _returnvalue))))

(event `self.Box.OnComponentEndOverlap`
  (params (OverlappedComponent :type "PrimitiveComponent Object Reference") (OtherActor :type "Actor Object Reference") (OtherComp :type "PrimitiveComponent Object Reference") (OtherBodyIndex :type Integer))
  (bind _asbp_car_base (cast `/Game/Core/Vehicles/BP_CarBase` OtherActor))
  (if (`KismetArrayLibrary.Array_Contains` (`self.AIArray`) _asbp_car_base)
    (set `/Game/Core/AI/BPC_AIControllerComponent.MaxSpeedMultiplier` 1.0 (`self.GetComponentByClass` _asbp_car_base "/Game/Core/AI/BPC_AIControllerComponent.BPC_AIControllerComponent_C"))))

(fn `UserConstructionScript`
  (`parent.UserConstructionScript`))