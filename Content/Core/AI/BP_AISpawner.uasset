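; BP_AISpawner spawns an AI-driven pawn of the configured Car class at its own location and rotation.
; It spawns only once, triggered by SpawnAI_Event or on BeginPlay when SpawnOnBeginPlay is set.
; It attaches a BPC AI controller component at runtime with the spawner's AISettings.
; That component receives a spline reference from SplineRoad, falling back to SplineTool.
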(event `SpawnAI_Event`
  (bind _splineroad (`self.SplineRoad`))
  (bind _splinetool (`self.SplineTool`))
  (`/Engine/EditorBlueprintResources/StandardMacros.DoOnce` false :!label _label
    (:`Completed`
      (bind _returnvalue (`AIBlueprintHelperLibrary.SpawnAIFromClass` (`self.Car`) null (`self.K2_GetActorLocation`) (`self.K2_GetActorRotation`) false null))
      (bind _returnvalue_2 (`AddComponent|NODE_AddBPC_AIControllerComponent-0` :`self` _returnvalue :`RelativeTransform` (`KismetMathLibrary.MakeTransform` (0.0 0.0 0.0)) :`AISettings` (`self.AISettings`)))
      (`/Engine/EditorBlueprintResources/StandardMacros.IsValid` _splineroad
        (:`Is Valid`
          (set `/Game/Core/AI/BPC_AIControllerComponent.SplineRef` (`/Game/Core/Objects/BP_SplineRoadTool.Spline` _splineroad) _returnvalue_2))
        (:`Is Not Valid`
          (`/Engine/EditorBlueprintResources/StandardMacros.IsValid` _splinetool
            (:`Is Valid`
              (set `/Game/Core/AI/BPC_AIControllerComponent.SplineRef` (`/Game/Core/Objects/SplineToolPro/Spline/SplineToolPro.Spline` _splinetool) _returnvalue_2))))))))

(event `self.ReceiveBeginPlay`
  (if (`self.SpawnOnBeginPlay`)
    (goto _label)))

(fn `UserConstructionScript`)