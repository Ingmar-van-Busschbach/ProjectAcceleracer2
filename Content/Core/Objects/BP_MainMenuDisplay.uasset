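; BP_MainMenuDisplay shows the player's currently selected car in the main menu.
; It caches GI_GlobalGameInstance on BeginPlay and polls its SelectedCar every Tick for changes.
; On a change, it destroys the previous car and spawns the new class at the SpawnLocation transform, muting its FMOD audio and enabling manual gear shifting on its engine component.
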(event `self.ReceiveBeginPlay`
  (bind _asgi_global_game_instance (cast `/Game/Core/GI_GlobalGameInstance` (`GameplayStatics.GetGameInstance`)))
  (set `self.GameInstance` _asgi_global_game_instance))

(event `self.ReceiveTick`
  (params (DeltaSeconds :type "Float (single-precision)"))
  (bind _selectedcar (`/Game/Core/GI_GlobalGameInstance.SelectedCar` (`self.GameInstance`)))
  (if (!= (`self.CarSelected`) _selectedcar)
    (set `self.CarSelected` _selectedcar)
    (`self.OnCarSelectedChanged`)))

(event `OnCarSelectedChanged`
  (bind _car (`self.Car`))
  (`/Engine/EditorBlueprintResources/StandardMacros.IsValid` _car
    (:`Is Valid`
      (`self.K2_DestroyActor` _car))
    (:`Is Not Valid`
      _))
  (bind _returnvalue (`|SpawnActorFromClass` (`self.CarSelected`) (`SceneComponent.K2_GetComponentToWorld` (`self.SpawnLocation`)) "AlwaysSpawn" "MultiplyWithRoot" null null))
  (bind _output_get (set `self.Car` _returnvalue))
  (`FMODAudioComponent.SetVolume` (`/Game/Core/Vehicles/BP_CarBase.FMODAudio` _output_get) 0.0)
  (set `/Game/Core/Vehicles/BP_EngineComponent.ManualGearShifting` true (`/Game/Core/Vehicles/BP_CarBase.BP_EngineComponent` _output_get)))

(fn `UserConstructionScript`)